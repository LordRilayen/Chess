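; BP_ChessPiece is a chess piece actor that positions itself on the board from integer grid coordinates.
; On BeginPlay it snaps to its CurrentLocation's X/Y at 100-unit spacing and fixed height, then registers itself as that location's CurrentPiece.
; A helper zeroes the directional movement counters and recentres the piece-mover widget.
; Pawn promotion is an unfinished, uncalled stub that only prints a placeholder message.
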(event `self.ReceiveBeginPlay`
  (`self.F_UpdatePiece`))

(fn `F_PromotePawnINCOMPLETE`
  (bind _currentlocation (`self.CurrentLocation`))
  (if (`self.IsBlack`)
    (if (`KismetArrayLibrary.Array_Contains` (`self.WhitePawnPromotionLocations`) _currentlocation)
      _
      (else
        _))
    (elif (`KismetArrayLibrary.Array_Contains` (`self.BlackPawnPromotionLocations`) _currentlocation)
      _
      (else
        _)))
  (`KismetSystemLibrary.PrintString` "Haven't Built Pawn Promotion Yet"))

(fn `F_ResetPieceMoverWidget`
  (set `self.MovementCounter_Right` 0)
  (set `self.MovementCounter_Left` 0)
  (set `self.MovementCounter_Up` 0)
  (set `self.MovementCounter_Down` 0)
  (`SceneComponent.K2_SetRelativeLocation` (`self.Widget`) (0.0 0.0 -2.9) false false))

(fn `F_SetCoordinates`
  (params (X :type Integer) (Y :type Integer))
  (bind _output_get (set `self.X` X))
  (bind _output_get_2 (set `self.Y` Y))
  (`self.K2_SetActorLocation` (`KismetMathLibrary.MakeVector` (`KismetMathLibrary.Conv_IntToDouble` (* _output_get 100)) (`KismetMathLibrary.Conv_IntToDouble` (* _output_get_2 100)) (`KismetMathLibrary.Conv_IntToDouble` 53))))

(fn `F_UpdatePiece`
  (bind _currentlocation (`self.CurrentLocation`))
  (`self.F_SetCoordinates` (`/Game/ActorBlueprints/BP_GridLocation.X` _currentlocation) (`/Game/ActorBlueprints/BP_GridLocation.Y` _currentlocation))
  (set `/Game/ActorBlueprints/BP_GridLocation.CurrentPiece` self (`self.CurrentLocation`)))

(fn `UserConstructionScript`)