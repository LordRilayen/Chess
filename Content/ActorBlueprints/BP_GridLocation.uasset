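; BP_GridLocation is a grid cell actor that can be selected and highlighted with a glow material.
; The construction script scales it by Width, Depth and Height, places it at its X/Y coordinates in 100-unit steps, and applies the glow if selected.
; FSelectLocation toggles selection and swaps to BasicShapeMaterial when deselected.
; The SetGridLocationSelection event refreshes the surface material from IsSelected, using DefaultMaterial when unselected.
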(event `self.ReceiveTick`
  (params (DeltaSeconds :type "Float (single-precision)")))

(event `SetGridLocationSelection`
  (`self.F_SetSelectionMaterial`))

(fn `F_SelectLocation`
  (bind _output_get (set `self.IsSelected` (not (`self.IsSelected`))))
  (if _output_get
    (`PrimitiveComponent.SetMaterial` (`self.Surface`) 0 "/Game/Materials/M_Selection_Glow.M_Selection_Glow")
    (else
      (`PrimitiveComponent.SetMaterial` (`self.Surface`) 0 "/Engine/BasicShapes/BasicShapeMaterial.BasicShapeMaterial"))))

(fn `F_SetCoordinates`
  (params (X :type Integer) (Y :type Integer))
  (`self.K2_SetActorLocation` (`KismetMathLibrary.MakeVector` (`KismetMathLibrary.Conv_IntToDouble` (* X 100)) (`KismetMathLibrary.Conv_IntToDouble` (* Y 100)) (`KismetMathLibrary.Conv_IntToDouble` 0))))

(fn `F_SetSelectionMaterial`
  (bind _surface (`self.Surface`))
  (if (`self.IsSelected`)
    (`PrimitiveComponent.SetMaterial` _surface 0 "/Game/Materials/M_Selection_Glow.M_Selection_Glow")
    (else
      (`PrimitiveComponent.SetMaterial` _surface 0 (`self.DefaultMaterial`)))))

(fn `UserConstructionScript`
  (bind _isselected (`self.IsSelected`))
  (`self.SetActorScale3D` (`KismetMathLibrary.MakeVector` (`KismetMathLibrary.Conv_IntToDouble` (`self.Width`)) (`KismetMathLibrary.Conv_IntToDouble` (`self.Depth`)) (`KismetMathLibrary.Conv_IntToDouble` (`self.Height`))))
  (`self.F_SetCoordinates` (`self.X`) (`self.Y`))
  (`KismetSystemLibrary.PrintString` (`KismetStringLibrary.Conv_BoolToString` _isselected))
  (if _isselected
    (`PrimitiveComponent.SetMaterial` (`self.Surface`) 0 "/Game/Materials/M_Selection_Glow.M_Selection_Glow")))