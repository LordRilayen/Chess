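; Knight chess piece Blueprint that extends a parent piece class with selection highlighting, movement and capture on a GameBoard.
; FUpdatePiece gathers its mesh parts and swaps their material between selection glow and default, showing the widget when selected.
; FMovePiece resolves the target square and calls FTakePiece, which validates the L-shape from directional counters, destroys enemies or flags self-selection and illegal moves.
; It then updates board occupancy and selection, and resets movement limits.
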(fn `F_CheckKnightL`
  (returns (HasKnightCompletedL :type Boolean))
  (return (and (or (== (`self.MovementCounter_Up`) 2) (== (`self.MovementCounter_Down`) 2) (== (`self.MovementCounter_Left`) 2) (== (`self.MovementCounter_Right`) 2)) (or (== (`self.MovementCounter_Up`) 1) (== (`self.MovementCounter_Down`) 1) (== (`self.MovementCounter_Left`) 1) (== (`self.MovementCounter_Right`) 1)))))

(fn `F_MovePiece`
  (params (`Target X` :type Integer) (`Target Y` :type Integer))
  (bind _gameboard (`self.GameBoard`))
  (bind _targetlocation (`self.TargetLocation`))
  (bind _gameboard_2 (`self.GameBoard`))
  (`parent.F_MovePiece` 0 0)
  (bind _grid_location (`/Game/ActorBlueprints/BP_GameBoard.GetMapLocationAtCoordinates` (`self.GameBoard`) `Target X` `Target Y`))
  (bind _output_get (set `self.TargetLocation` _grid_location))
  (`self.F_TakePiece` _output_get)
  (if (`self.IsSelfSelecting`)
    (set `self.IsSelected` false)
    (`SceneComponent.SetVisibility` (`/Game/ActorBlueprints/BP_ChessPiece.Widget` (stale _output_get_3)) false false :!label _label)
    (`self.F_UpdatePiece` (stale _output_get_3))
    (bind _output_get_2 (set `/Game/ActorBlueprints/BP_GameBoard.SelectedLocation` (`self.TargetLocation`) (`self.GameBoard`)))
    (set `/Game/ActorBlueprints/BP_GridLocation.IsSelected` true _output_get_2)
    (`/Game/ActorBlueprints/BP_GridLocation.F_SetSelectionMaterial` _output_get_2)
    (set `/Game/ActorBlueprints/BP_GameBoard.SelectedLocationIndex` (`KismetArrayLibrary.Array_Find` (`/Game/ActorBlueprints/BP_GameBoard.MapLocations` _gameboard_2) _output_get_2) _gameboard_2)
    (if (`self.isSelfSelecting`)
      (set `self.isSelfSelecting` false))
    (elif (`self.isTakeAllowed`)
      (bind _output_get_3 (set `/Game/ActorBlueprints/BP_GridLocation.CurrentPiece` self _targetlocation))
      (set `/Game/ActorBlueprints/BP_ChessPiece.IsSelected` false _output_get_3)
      (set `/Game/ActorBlueprints/BP_GridLocation.CurrentPiece` null (`/Game/ActorBlueprints/BP_GameBoard.SelectedLocation` (`self.GameBoard`))) ; Gotta find the right place to put this to not break self-selection
      (set `/Game/ActorBlueprints/BP_ChessPiece.CurrentLocation` _targetlocation _output_get_3)
      (goto _label)
      (else
        (set `self.isTakeAllowed` true)
        (set `self.IsSelected` false)
        (`SceneComponent.SetVisibility` (`self.Widget`) false false)
        (`self.F_UpdatePiece` self)
        (bind _output_get_4 (set `/Game/ActorBlueprints/BP_GameBoard.SelectedLocation` (`self.CurrentLocation`) (`self.GameBoard`)))
        (set `/Game/ActorBlueprints/BP_GridLocation.IsSelected` true _output_get_4)
        (`/Game/ActorBlueprints/BP_GridLocation.F_SetSelectionMaterial` _output_get_4)
        (set `/Game/ActorBlueprints/BP_GameBoard.SelectedLocationIndex` (`KismetArrayLibrary.Array_Find` (`/Game/ActorBlueprints/BP_GameBoard.MapLocations` _gameboard) _output_get_4) _gameboard))))
  (set `self.MovementLimit_Left` 2)
  (set `self.MovementLimit_Right` 2)
  (set `self.MovementLimit_Up` 2)
  (set `self.MovementLimit_Down` 2))

(fn `F_TakePiece`
  (params (InputLocation :type "/Game/ActorBlueprints/BP_GridLocation Object Reference"))
  (bind _currentpiece (`/Game/ActorBlueprints/BP_GridLocation.CurrentPiece` InputLocation))
  (`parent.F_TakePiece` null)
  (bind _hasknightcompletedl (`self.F_CheckKnightL`))
  (if _hasknightcompletedl
    (if (`KismetSystemLibrary.IsValid` _currentpiece)
      (if (== _currentpiece self)
        (set `self.IsSelfSelecting` true)
        (elif (!= (`/Game/ActorBlueprints/BP_ChessPiece.IsBlack` _currentpiece) (`self.IsBlack`))
          (`self.K2_DestroyActor` _currentpiece)
          (else
            (set `self.isTakeAllowed` false :!label _label)))))
    (else
      (goto _label))))

(fn `F_UpdateKnightPieceINCOMPLETE`
  (if (`self.IsSelected`)
    (for _array_element (`self.AllComponents`)
      (`PrimitiveComponent.SetMaterial` _array_element 0 "/Game/Materials/M_Selection_Glow.M_Selection_Glow"))
    (`SceneComponent.SetVisibility` (`self.Widget`) true false)
    (else
      (for _array_element_2 (`self.AllComponents`)
        (`PrimitiveComponent.SetMaterial` _array_element_2 0 (`self.DefaultMaterial`))))))

(fn `F_UpdatePiece`
  (bind _allcomponents (`self.AllComponents`))
  (`parent.F_UpdatePiece`)
  (if (== (`KismetArrayLibrary.Array_Length` (`self.AllComponents`)) 0)
    (`KismetArrayLibrary.Array_Add` _allcomponents (`self.Ear2`))
    (`KismetArrayLibrary.Array_Add` _allcomponents (`self.Ear1`))
    (`KismetArrayLibrary.Array_Add` _allcomponents (`self.Nose2`))
    (`KismetArrayLibrary.Array_Add` _allcomponents (`self.Nose1`))
    (`KismetArrayLibrary.Array_Add` _allcomponents (`self.Head`))
    (`KismetArrayLibrary.Array_Add` _allcomponents (`self.Neck4`))
    (`KismetArrayLibrary.Array_Add` _allcomponents (`self.Neck3`))
    (`KismetArrayLibrary.Array_Add` _allcomponents (`self.Neck2`))
    (`KismetArrayLibrary.Array_Add` _allcomponents (`self.Neck1`))
    (`KismetArrayLibrary.Array_Add` _allcomponents (`self.Pedestal`))
    (`KismetArrayLibrary.Array_Add` _allcomponents (`self.Base`)))
  (`self.F_UpdateKnightPieceINCOMPLETE`))

(fn `UserConstructionScript`
  (`parent.UserConstructionScript`))