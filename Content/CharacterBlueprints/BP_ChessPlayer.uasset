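; Player Blueprint for keyboard-controlled checkers, despite the chess name, with movement and look input disabled.
; Arrow keys move either the BP_GameBoard square selection or the chosen piece's mover widget within its limits, with Right Ctrl selecting and confirming.
; Confirming accepts dark squares, deselects on the piece's own square, or jumps an opposing piece if the square beyond is free.
; Jump direction comes from switching on the four movement counters joined as a string.
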(event `Key|Q`
  (params (Key :type "Key Structure")))

(event `Key|W`
  (params (Key :type "Key Structure")))

(event `Key|E`
  (params (Key :type "Key Structure")))

(event `Key|Escape`
  (params (Key :type "Key Structure"))
  (:`Pressed`
    (`KismetSystemLibrary.QuitGame` null "Quit")))

(event `self.ReceiveBeginPlay`
  (`self.SetIgnoreMoveInput` true)
  (`self.SetIgnoreLookInput` true))

(event `Key|Up`
  (params (Key :type "Key Structure"))
  (:`Pressed`
    (if (`self.AreSelectingLocation`)
      (`self.F_MoveSelectionUp`)
      (elif (`self.AreSelectingAction`)
        (`self.F_MovePieceSelectionUp`)))))

(event `Key|Left`
  (params (Key :type "Key Structure"))
  (:`Pressed`
    (if (`self.AreSelectingLocation`)
      (`self.F_MoveSelectionLeft`)
      (elif (`self.AreSelectingAction`)
        (`self.F_MovePieceSelectionLeft`)))))

(event `Key|Down`
  (params (Key :type "Key Structure"))
  (:`Pressed`
    (if (`self.AreSelectingLocation`)
      (`self.F_MoveSelectionDown`)
      (elif (`self.AreSelectingAction`)
        (`self.F_MovePieceSelectionDown`)))))

(event `Key|Right`
  (params (Key :type "Key Structure"))
  (:`Pressed`
    (if (`self.AreSelectingLocation`)
      (`self.F_MoveSelectionRight`)
      (elif (`self.AreSelectingAction`)
        (`self.F_MovePieceSelectionRight`)))))

(event `Key|RightControl`
  (params (Key :type "Key Structure"))
  (:`Pressed`
    (if (`self.AreSelectingLocation`)
      (`self.F Begin Selecting Action` (`self.GameBoard`))
      (elif (`self.AreSelectingAction`)
        (`self.F_MoveChecker`)))))

(fn `F Begin Selecting Action`
  (params (GameBoard :type "/Game/ActorBlueprints/BP_GameBoard Object Reference"))
  (bind _selectedlocation (`/Game/ActorBlueprints/BP_GameBoard.SelectedLocation` (`self.GameBoard`)))
  (bind _currentpiece (`/Game/ActorBlueprints/BP_GridLocation.CurrentPiece` _selectedlocation))
  (set `self.AreSelectingLocation` false)
  (set `self.AreSelectingAction` true)
  (set `/Game/ActorBlueprints/BP_GridLocation.IsSelected` false _selectedlocation)
  (`/Game/ActorBlueprints/BP_GridLocation.SetGridLocationSelection` _selectedlocation)
  (set `/Game/ActorBlueprints/BP_ChessPiece.IsSelected` true _currentpiece)
  (`/Game/ActorBlueprints/BP_ChessPiece.F_UpdatePiece` _currentpiece)
  (set `self.Target_X` (`/Game/ActorBlueprints/BP_ChessPiece.X` _currentpiece))
  (set `self.Target_Y` (`/Game/ActorBlueprints/BP_ChessPiece.Y` _currentpiece))
  (`/Game/ActorBlueprints/BP_ChessPiece.F_ResetPieceMoverWidget` _currentpiece))

(fn `F_CheckDestination`
  (params (CurrentPiece :type "/Game/ActorBlueprints/BP_ChessPiece Object Reference"))
  (returns (isDestinationOccupied :type Boolean))
  (switch `string` (`KismetStringLibrary.Concat_StrStr` (`KismetStringLibrary.Conv_IntToString` (`/Game/ActorBlueprints/BP_ChessPiece.MovementCounter_Down` CurrentPiece)) "," (`KismetStringLibrary.Conv_IntToString` (`/Game/ActorBlueprints/BP_ChessPiece.MovementCounter_Left` CurrentPiece)) "," (`KismetStringLibrary.Conv_IntToString` (`/Game/ActorBlueprints/BP_ChessPiece.MovementCounter_Right` CurrentPiece)) "," (`KismetStringLibrary.Conv_IntToString` (`/Game/ActorBlueprints/BP_ChessPiece.MovementCounter_Up` CurrentPiece)))
    (:`-1,-1,1,1`
      (`self.F_CheckDestinationUp`)
      (`self.F_CheckDestinationRight`))
    (:`-1,1,-1,1`
      (`self.F_CheckDestinationUp`)
      (`self.F_CheckDestinationLeft`))
    (:`1,1,-1,-1`
      (`self.F_CheckDestinationDown`)
      (`self.F_CheckDestinationLeft`))
    (:`1,-1,1,-1`
      (`self.F_CheckDestinationDown`)
      (`self.F_CheckDestinationRight`)))
  (if (`/Game/ActorBlueprints/BP_GridLocation.isBlack` (`self.DestinationQueryLocation`))
    (return (`KismetSystemLibrary.IsValid` (`/Game/ActorBlueprints/BP_GridLocation.CurrentPiece` (`self.DestinationQueryLocation`))))
    (else
      (return true) ; If the location isn't black, that means the movement checked something out of bounds. For the purposes of taking a piece, this is also invalid, so return as if the function found a piece in the destination.
    )))

(fn `F_CheckDestinationDown`
  (bind _destinationquerylocation (`self.DestinationQueryLocation`))
  (bind _grid_location (`/Game/ActorBlueprints/BP_GameBoard.GetMapLocationAtCoordinates` (`self.GameBoard`) (- (`/Game/ActorBlueprints/BP_GridLocation.X` _destinationquerylocation) 1) (`/Game/ActorBlueprints/BP_GridLocation.Y` _destinationquerylocation)))
  (if (`KismetSystemLibrary.IsValid` _grid_location)
    (set `self.DestinationQueryLocation` _grid_location)))

(fn `F_CheckDestinationLeft`
  (bind _destinationquerylocation (`self.DestinationQueryLocation`))
  (bind _grid_location (`/Game/ActorBlueprints/BP_GameBoard.GetMapLocationAtCoordinates` (`self.GameBoard`) (`/Game/ActorBlueprints/BP_GridLocation.X` _destinationquerylocation) (- (`/Game/ActorBlueprints/BP_GridLocation.Y` _destinationquerylocation) 1)))
  (if (`KismetSystemLibrary.IsValid` _grid_location)
    (set `self.DestinationQueryLocation` _grid_location)))

(fn `F_CheckDestinationRight`
  (bind _destinationquerylocation (`self.DestinationQueryLocation`))
  (bind _grid_location (`/Game/ActorBlueprints/BP_GameBoard.GetMapLocationAtCoordinates` (`self.GameBoard`) (`/Game/ActorBlueprints/BP_GridLocation.X` _destinationquerylocation) (+ (`/Game/ActorBlueprints/BP_GridLocation.Y` _destinationquerylocation) 1)))
  (if (`KismetSystemLibrary.IsValid` _grid_location)
    (set `self.DestinationQueryLocation` _grid_location)))

(fn `F_CheckDestinationUp`
  (bind _destinationquerylocation (`self.DestinationQueryLocation`))
  (bind _grid_location (`/Game/ActorBlueprints/BP_GameBoard.GetMapLocationAtCoordinates` (`self.GameBoard`) (+ (`/Game/ActorBlueprints/BP_GridLocation.X` _destinationquerylocation) 1) (`/Game/ActorBlueprints/BP_GridLocation.Y` _destinationquerylocation)))
  (if (`KismetSystemLibrary.IsValid` _grid_location)
    (set `self.DestinationQueryLocation` _grid_location)))

(fn `F_MoveChecker`
  (bind _gameboard (`self.GameBoard`))
  (bind _targetlocation (`self.TargetLocation`))
  (bind _currentpiece (`/Game/ActorBlueprints/BP_GridLocation.CurrentPiece` (`/Game/ActorBlueprints/BP_GameBoard.SelectedLocation` (`self.GameBoard`))))
  (bind _grid_location (`/Game/ActorBlueprints/BP_GameBoard.GetMapLocationAtCoordinates` (`self.GameBoard`) (`self.Target_X`) (`self.Target_Y`)))
  (bind _output_get (set `self.TargetLocation` _grid_location))
  (set `self.DestinationQueryLocation` _output_get)
  (`self.F_TakePiece` _output_get _currentpiece)
  (if (`self.IsSelfSelecting`)
    (set `self.IsSelfSelecting` false)
    (set `/Game/ActorBlueprints/BP_ChessPiece.IsSelected` false (stale _output_get_3))
    (`SceneComponent.SetVisibility` (`/Game/ActorBlueprints/BP_ChessPiece.Widget` (stale _output_get_3)) false false :!label _label)
    (`/Game/ActorBlueprints/BP_ChessPiece.F_UpdatePiece` (stale _output_get_3))
    (set `self.AreSelectingLocation` true)
    (set `self.AreSelectingAction` false)
    (bind _output_get_2 (set `/Game/ActorBlueprints/BP_GameBoard.SelectedLocation` (`self.TargetLocation`) (`self.GameBoard`)))
    (set `/Game/ActorBlueprints/BP_GridLocation.IsSelected` true _output_get_2)
    (`/Game/ActorBlueprints/BP_GridLocation.F_SetSelectionMaterial` _output_get_2)
    (set `/Game/ActorBlueprints/BP_GameBoard.SelectedLocationIndex` (`KismetArrayLibrary.Array_Find` (`/Game/ActorBlueprints/BP_GameBoard.MapLocations` _gameboard) _output_get_2) _gameboard)
    (elif (`self.isTakeAllowed`)
      (if (`/Game/ActorBlueprints/BP_GridLocation.isBlack` _targetlocation)
        (bind _output_get_3 (set `/Game/ActorBlueprints/BP_GridLocation.CurrentPiece` _currentpiece _targetlocation))
        (set `/Game/ActorBlueprints/BP_ChessPiece.IsSelected` false _output_get_3)
        (set `/Game/ActorBlueprints/BP_GridLocation.CurrentPiece` null (`/Game/ActorBlueprints/BP_GameBoard.SelectedLocation` (`self.GameBoard`))) ; Gotta find the right place to put this to not break self-selection
        (set `/Game/ActorBlueprints/BP_ChessPiece.CurrentLocation` _targetlocation _output_get_3)
        (goto _label))
      (else
        (set `self.isTakeAllowed` true)))))

(fn `F_MovePieceSelectionDown`
  (bind _currentpiece (`/Game/ActorBlueprints/BP_GridLocation.CurrentPiece` (`/Game/ActorBlueprints/BP_GameBoard.SelectedLocation` (`self.GameBoard`))))
  (bind _returnvalue (`self.GetComponentByClass` _currentpiece "/Script/UMG.WidgetComponent"))
  (if (not (== (`/Game/ActorBlueprints/BP_ChessPiece.MovementCounter_Down` _currentpiece) (`/Game/ActorBlueprints/BP_ChessPiece.MovementLimit_Down` _currentpiece)))
    (`SceneComponent.K2_SetWorldLocation` _returnvalue (`KismetMathLibrary.MakeVector` (- (.x (`SceneComponent.K2_GetComponentLocation` _returnvalue)) 100.0) (.y (`SceneComponent.K2_GetComponentLocation` _returnvalue)) (.z (`SceneComponent.K2_GetComponentLocation` _returnvalue))) false false)
    (`/Engine/EditorBlueprintResources/StandardMacros.IncrementInt` (`/Game/ActorBlueprints/BP_ChessPiece.MovementCounter_Down` _currentpiece)
      (:`  `
        (`/Engine/EditorBlueprintResources/StandardMacros.DecrementInt` (`/Game/ActorBlueprints/BP_ChessPiece.MovementCounter_Up` _currentpiece)
          (:`  `
            (`/Engine/EditorBlueprintResources/StandardMacros.DecrementInt` (`self.Target_X`))))))))

(fn `F_MovePieceSelectionLeft`
  (bind _currentpiece (`/Game/ActorBlueprints/BP_GridLocation.CurrentPiece` (`/Game/ActorBlueprints/BP_GameBoard.SelectedLocation` (`self.GameBoard`))))
  (bind _returnvalue (`self.GetComponentByClass` _currentpiece "/Script/UMG.WidgetComponent"))
  (if (not (== (`/Game/ActorBlueprints/BP_ChessPiece.MovementCounter_Left` _currentpiece) (`/Game/ActorBlueprints/BP_ChessPiece.MovementLimit_Left` _currentpiece)))
    (`SceneComponent.K2_SetWorldLocation` _returnvalue (`KismetMathLibrary.MakeVector` (.x (`SceneComponent.K2_GetComponentLocation` _returnvalue)) (- (.y (`SceneComponent.K2_GetComponentLocation` _returnvalue)) 100.0) (.z (`SceneComponent.K2_GetComponentLocation` _returnvalue))) false false)
    (`/Engine/EditorBlueprintResources/StandardMacros.IncrementInt` (`/Game/ActorBlueprints/BP_ChessPiece.MovementCounter_Left` _currentpiece)
      (:`  `
        (`/Engine/EditorBlueprintResources/StandardMacros.DecrementInt` (`/Game/ActorBlueprints/BP_ChessPiece.MovementCounter_Right` _currentpiece)
          (:`  `
            (`/Engine/EditorBlueprintResources/StandardMacros.DecrementInt` (`self.Target_Y`))))))))

(fn `F_MovePieceSelectionRight`
  (bind _currentpiece (`/Game/ActorBlueprints/BP_GridLocation.CurrentPiece` (`/Game/ActorBlueprints/BP_GameBoard.SelectedLocation` (`self.GameBoard`))))
  (bind _returnvalue (`self.GetComponentByClass` _currentpiece "/Script/UMG.WidgetComponent"))
  (if (not (== (`/Game/ActorBlueprints/BP_ChessPiece.MovementCounter_Right` _currentpiece) (`/Game/ActorBlueprints/BP_ChessPiece.MovementLimit_Right` _currentpiece)))
    (`SceneComponent.K2_SetWorldLocation` _returnvalue (`KismetMathLibrary.MakeVector` (.x (`SceneComponent.K2_GetComponentLocation` _returnvalue)) (+ (.y (`SceneComponent.K2_GetComponentLocation` _returnvalue)) 100.0) (.z (`SceneComponent.K2_GetComponentLocation` _returnvalue))) false false)
    (`/Engine/EditorBlueprintResources/StandardMacros.IncrementInt` (`/Game/ActorBlueprints/BP_ChessPiece.MovementCounter_Right` _currentpiece)
      (:`  `
        (`/Engine/EditorBlueprintResources/StandardMacros.DecrementInt` (`/Game/ActorBlueprints/BP_ChessPiece.MovementCounter_Left` _currentpiece)
          (:`  `
            (`/Engine/EditorBlueprintResources/StandardMacros.IncrementInt` (`self.Target_Y`))))))))

(fn `F_MovePieceSelectionUp`
  (bind _currentpiece (`/Game/ActorBlueprints/BP_GridLocation.CurrentPiece` (`/Game/ActorBlueprints/BP_GameBoard.SelectedLocation` (`self.GameBoard`))))
  (bind _returnvalue (`self.GetComponentByClass` _currentpiece "/Script/UMG.WidgetComponent"))
  (if (not (== (`/Game/ActorBlueprints/BP_ChessPiece.MovementCounter_Up` _currentpiece) (`/Game/ActorBlueprints/BP_ChessPiece.MovementLimit_Up` _currentpiece)))
    (`SceneComponent.K2_SetWorldLocation` _returnvalue (`KismetMathLibrary.MakeVector` (+ (.x (`SceneComponent.K2_GetComponentLocation` _returnvalue)) 100.0) (.y (`SceneComponent.K2_GetComponentLocation` _returnvalue)) (.z (`SceneComponent.K2_GetComponentLocation` _returnvalue))) false false)
    (`/Engine/EditorBlueprintResources/StandardMacros.IncrementInt` (`/Game/ActorBlueprints/BP_ChessPiece.MovementCounter_Up` _currentpiece)
      (:`  `
        (`/Engine/EditorBlueprintResources/StandardMacros.DecrementInt` (`/Game/ActorBlueprints/BP_ChessPiece.MovementCounter_Down` _currentpiece)
          (:`  `
            (`/Engine/EditorBlueprintResources/StandardMacros.IncrementInt` (`self.Target_X`))))))))

(fn `F_MoveSelectionDown`
  (bind _gameboard (`self.GameBoard`))
  (bind _gameboard_2 (`self.GameBoard`))
  (bind _selectedlocation (`/Game/ActorBlueprints/BP_GameBoard.SelectedLocation` (`self.GameBoard`)))
  (bind _selectedlocation_2 (`/Game/ActorBlueprints/BP_GameBoard.SelectedLocation` (`self.GameBoard`)))
  (if (> (`/Game/ActorBlueprints/BP_GridLocation.X` (`/Game/ActorBlueprints/BP_GameBoard.SelectedLocation` (`self.GameBoard`))) 0)
    (set `/Game/ActorBlueprints/BP_GridLocation.IsSelected` false _selectedlocation_2)
    (`/Game/ActorBlueprints/BP_GridLocation.SetGridLocationSelection` _selectedlocation_2)
    (bind _output_get (set `/Game/ActorBlueprints/BP_GameBoard.SelectedLocationIndex` (- (`/Game/ActorBlueprints/BP_GameBoard.SelectedLocationIndex` _gameboard_2) 8) _gameboard_2))
    (bind _output_get_2 (set `/Game/ActorBlueprints/BP_GameBoard.SelectedLocation` (`|GetArrayItem` (`/Game/ActorBlueprints/BP_GameBoard.MapLocations` _gameboard) _output_get) _gameboard))
    (`/Game/ActorBlueprints/BP_GridLocation.SetGridLocationSelection` _output_get_2)
    (bind _output_get_3 (set `/Game/ActorBlueprints/BP_GameBoard.SelectedLocation` _output_get_2 (`self.GameBoard`)))
    (`/Game/ActorBlueprints/BP_GridLocation.SetGridLocationSelection` _output_get_3)
    (set `/Game/ActorBlueprints/BP_GridLocation.IsSelected` true _selectedlocation)
    (`/Game/ActorBlueprints/BP_GridLocation.SetGridLocationSelection` _selectedlocation)))

(fn `F_MoveSelectionLeft`
  (bind _gameboard (`self.GameBoard`))
  (bind _selectedlocation (`/Game/ActorBlueprints/BP_GameBoard.SelectedLocation` (`self.GameBoard`)))
  (bind _selectedlocation_2 (`/Game/ActorBlueprints/BP_GameBoard.SelectedLocation` (`self.GameBoard`)))
  (if (> (`/Game/ActorBlueprints/BP_GridLocation.Y` (`/Game/ActorBlueprints/BP_GameBoard.SelectedLocation` (`self.GameBoard`))) 0)
    (set `/Game/ActorBlueprints/BP_GridLocation.IsSelected` false _selectedlocation_2)
    (`/Game/ActorBlueprints/BP_GridLocation.SetGridLocationSelection` _selectedlocation_2)
    (bind _result (`/Engine/EditorBlueprintResources/StandardMacros.DecrementInt` (`/Game/ActorBlueprints/BP_GameBoard.SelectedLocationIndex` (`self.GameBoard`)))
      (:`  `
        (bind _output_get (set `/Game/ActorBlueprints/BP_GameBoard.SelectedLocation` (`|GetArrayItem` (`/Game/ActorBlueprints/BP_GameBoard.MapLocations` _gameboard) _result) _gameboard))
        (`/Game/ActorBlueprints/BP_GridLocation.SetGridLocationSelection` _output_get)
        (bind _output_get_2 (set `/Game/ActorBlueprints/BP_GameBoard.SelectedLocation` _output_get (`self.GameBoard`)))
        (`/Game/ActorBlueprints/BP_GridLocation.SetGridLocationSelection` _output_get_2)
        (set `/Game/ActorBlueprints/BP_GridLocation.IsSelected` true _selectedlocation)
        (`/Game/ActorBlueprints/BP_GridLocation.SetGridLocationSelection` _selectedlocation)))))

(fn `F_MoveSelectionRight`
  (bind _gameboard (`self.GameBoard`))
  (bind _selectedlocation (`/Game/ActorBlueprints/BP_GameBoard.SelectedLocation` (`self.GameBoard`)))
  (bind _selectedlocation_2 (`/Game/ActorBlueprints/BP_GameBoard.SelectedLocation` (`self.GameBoard`)))
  (if (< (`/Game/ActorBlueprints/BP_GridLocation.Y` (`/Game/ActorBlueprints/BP_GameBoard.SelectedLocation` (`self.GameBoard`))) 7)
    (set `/Game/ActorBlueprints/BP_GridLocation.IsSelected` false _selectedlocation_2)
    (`/Game/ActorBlueprints/BP_GridLocation.SetGridLocationSelection` _selectedlocation_2)
    (bind _result (`/Engine/EditorBlueprintResources/StandardMacros.IncrementInt` (`/Game/ActorBlueprints/BP_GameBoard.SelectedLocationIndex` (`self.GameBoard`)))
      (:`  `
        (bind _output_get (set `/Game/ActorBlueprints/BP_GameBoard.SelectedLocation` (`|GetArrayItem` (`/Game/ActorBlueprints/BP_GameBoard.MapLocations` _gameboard) _result) _gameboard))
        (`/Game/ActorBlueprints/BP_GridLocation.SetGridLocationSelection` _output_get)
        (bind _output_get_2 (set `/Game/ActorBlueprints/BP_GameBoard.SelectedLocation` _output_get (`self.GameBoard`)))
        (`/Game/ActorBlueprints/BP_GridLocation.SetGridLocationSelection` _output_get_2)
        (set `/Game/ActorBlueprints/BP_GridLocation.IsSelected` true _selectedlocation)
        (`/Game/ActorBlueprints/BP_GridLocation.SetGridLocationSelection` _selectedlocation)))))

(fn `F_MoveSelectionUp`
  (bind _gameboard (`self.GameBoard`))
  (bind _gameboard_2 (`self.GameBoard`))
  (bind _selectedlocation (`/Game/ActorBlueprints/BP_GameBoard.SelectedLocation` (`self.GameBoard`)))
  (bind _selectedlocation_2 (`/Game/ActorBlueprints/BP_GameBoard.SelectedLocation` (`self.GameBoard`)))
  (if (< (`/Game/ActorBlueprints/BP_GridLocation.X` (`/Game/ActorBlueprints/BP_GameBoard.SelectedLocation` (`self.GameBoard`))) 7)
    (set `/Game/ActorBlueprints/BP_GridLocation.IsSelected` false _selectedlocation_2)
    (`/Game/ActorBlueprints/BP_GridLocation.SetGridLocationSelection` _selectedlocation_2)
    (bind _output_get (set `/Game/ActorBlueprints/BP_GameBoard.SelectedLocationIndex` (+ (`/Game/ActorBlueprints/BP_GameBoard.SelectedLocationIndex` _gameboard_2) 8) _gameboard_2))
    (bind _output_get_2 (set `/Game/ActorBlueprints/BP_GameBoard.SelectedLocation` (`|GetArrayItem` (`/Game/ActorBlueprints/BP_GameBoard.MapLocations` _gameboard) _output_get) _gameboard))
    (`/Game/ActorBlueprints/BP_GridLocation.SetGridLocationSelection` _output_get_2)
    (bind _output_get_3 (set `/Game/ActorBlueprints/BP_GameBoard.SelectedLocation` _output_get_2 (`self.GameBoard`)))
    (`/Game/ActorBlueprints/BP_GridLocation.SetGridLocationSelection` _output_get_3)
    (set `/Game/ActorBlueprints/BP_GridLocation.IsSelected` true _selectedlocation)
    (`/Game/ActorBlueprints/BP_GridLocation.SetGridLocationSelection` _selectedlocation)))

(fn `F_ResetCounters`
  (params (`Chess Piece` :type "/Game/ActorBlueprints/BP_ChessPiece Object Reference"))
  (set `/Game/ActorBlueprints/BP_ChessPiece.MovementCounter_Down` 0 `Chess Piece`)
  (set `/Game/ActorBlueprints/BP_ChessPiece.MovementCounter_Left` 0 `Chess Piece`)
  (set `/Game/ActorBlueprints/BP_ChessPiece.MovementCounter_Right` 0 `Chess Piece`)
  (set `/Game/ActorBlueprints/BP_ChessPiece.MovementCounter_Up` 0 `Chess Piece`))

(fn `F_TakePiece`
  (params (InputLocation :type "/Game/ActorBlueprints/BP_GridLocation Object Reference") (CurrentPiece :type "/Game/ActorBlueprints/BP_ChessPiece Object Reference"))
  (bind _currentpiece (`/Game/ActorBlueprints/BP_GridLocation.CurrentPiece` InputLocation))
  (if (`KismetSystemLibrary.IsValid` _currentpiece)
    (if (== _currentpiece CurrentPiece)
      (set `self.IsSelfSelecting` true)
      (else
        (bind _isdestinationoccupied (`self.F_CheckDestination` CurrentPiece))
        (if _isdestinationoccupied
          (set `self.isTakeAllowed` false :!label _label)
          (elif (!= (`/Game/ActorBlueprints/BP_ChessPiece.IsBlack` _currentpiece) (`/Game/ActorBlueprints/BP_ChessPiece.IsBlack` CurrentPiece))
            (`self.K2_DestroyActor` (`/Game/ActorBlueprints/BP_GridLocation.CurrentPiece` InputLocation))
            (switch `string` (`KismetStringLibrary.Concat_StrStr` (`KismetStringLibrary.Conv_IntToString` (`/Game/ActorBlueprints/BP_ChessPiece.MovementCounter_Down` CurrentPiece)) "," (`KismetStringLibrary.Conv_IntToString` (`/Game/ActorBlueprints/BP_ChessPiece.MovementCounter_Left` CurrentPiece)) "," (`KismetStringLibrary.Conv_IntToString` (`/Game/ActorBlueprints/BP_ChessPiece.MovementCounter_Right` CurrentPiece)) "," (`KismetStringLibrary.Conv_IntToString` (`/Game/ActorBlueprints/BP_ChessPiece.MovementCounter_Up` CurrentPiece)))
              (:`-1,-1,1,1`
                (`self.F_ResetCounters` CurrentPiece)
                (`self.F_MovePieceSelectionUp`)
                (`self.F_MovePieceSelectionRight`))
              (:`-1,1,-1,1`
                (`self.F_ResetCounters` CurrentPiece)
                (`self.F_MovePieceSelectionUp`)
                (`self.F_MovePieceSelectionLeft`))
              (:`1,1,-1,-1`
                (`self.F_ResetCounters` CurrentPiece)
                (`self.F_MovePieceSelectionDown`)
                (`self.F_MovePieceSelectionLeft`))
              (:`1,-1,1,-1`
                (`self.F_ResetCounters` CurrentPiece)
                (`self.F_MovePieceSelectionDown`)
                (`self.F_MovePieceSelectionRight`)))
            (bind _grid_location (`/Game/ActorBlueprints/BP_GameBoard.GetMapLocationAtCoordinates` (`self.GameBoard`) (`self.Target_X`) (`self.Target_Y`)))
            (set `self.TargetLocation` _grid_location)
            (else
              (goto _label))))))))

(fn `UserConstructionScript`
  (bind _returnvalue (`GameplayStatics.GetActorOfClass` "/Game/ActorBlueprints/BP_GameBoard.BP_GameBoard_C"))
  (set `self.GameBoard` _returnvalue))